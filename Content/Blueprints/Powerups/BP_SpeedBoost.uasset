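; Speed boost powerup that doubles the walk speed of the actor that picks it up until it expires.
; Activation and expiry call the parent, then double or halve the CharacterMovementComponent's current max speed into NewSpeed, if that component exists.
; NewSpeed is a RepNotify variable whose OnRep writes MaxWalkSpeed, so the change replicates.
; Expiry halves whatever the speed is then, rather than restoring a saved original.
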(event EventOnActivating
  (params (PickingUpActor :type Actor%20Object%20Reference))
  (bind _picking_up_actor (Variables|Default|GetPicking%20Up%20Actor))
  (bind _returnvalue (Actor|GetComponentbyClass _picking_up_actor "/Script/Engine.CharacterMovementComponent"))
  (|CallParentFunction PickingUpActor)
  (Utilities|IsValid _picking_up_actor
    (:Is%20Valid
      (Utilities|IsValid _returnvalue
        (:Is%20Valid
          (Variables|Default|SetNewSpeed (* (Class|MovementComponent|GetMaxSpeed _returnvalue) 2.0)))))))

(event EventOnExpiring
  (bind _picking_up_actor (Variables|Default|GetPicking%20Up%20Actor))
  (bind _returnvalue (Actor|GetComponentbyClass _picking_up_actor "/Script/Engine.CharacterMovementComponent"))
  (|CallParentFunction)
  (Utilities|IsValid _picking_up_actor
    (:Is%20Valid
      (Utilities|IsValid _returnvalue
        (:Is%20Valid
          (Variables|Default|SetNewSpeed (/ (Class|MovementComponent|GetMaxSpeed _returnvalue) 2.0)))))))

(fn ConstructionScript)

(fn OnRepNewSpeed
  (Variables|/Script/Engine.CharacterMovementComponent|SetMaxWalkSpeed (Actor|GetComponentbyClass (Variables|Default|GetPicking%20Up%20Actor) "/Script/Engine.CharacterMovementComponent") (Variables|Default|GetNewSpeed)))