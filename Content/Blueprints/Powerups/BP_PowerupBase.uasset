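; Base powerup Blueprint that handles the visual, audio and lifetime responses to a powerup's lifecycle events.
; A state change sets the actor's hidden state from the event's flag, and activation stores the picking-up actor and plays the pickup sound.
; Each tick event plays the active sound at the actor's location, and expiry sets a short lifespan so the actor destroys itself.
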(event EventOnPowerupTicked
  (Audio|PlaySoundatLocation (Variables|Powerups|GetActiveSound) (Transformation|GetActorLocation) "0, 0, 0" 1.0 1.0 0.0 0 0 0))

(event EventOnPowerupStateChange
  (params (bIsPowerupStatedChanged :type Boolean))
  (Rendering|SetActorHiddenInGame bIsPowerupStatedChanged))

(event EventOnActivating
  (params (PickingUpActor :type Actor%20Object%20Reference))
  (Variables|Default|SetPicking%20Up%20Actor PickingUpActor)
  (Audio|PlaySoundatLocation (Variables|Powerups|GetPickupSound) (Transformation|GetActorLocation) "0, 0, 0" 1.0 1.0 0.0 0 0 0))

(event EventOnExpiring
  (Actor|SetLifeSpan 1.0))

(fn ConstructionScript)