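; Wave-based co-op game mode that spawns enemy bots and awards score for kills.
; SpawnNewBot runs an EQS spawn-location query, then spawns a BP_AdvanceAI or BP_TrackerBot at even odds at each returned location.
; Actor-killed events add the victim bot's KilledScore to the killer's COOP_PlayerState and print the total.
; Restarting a player creates that character's HUD.
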(event Custom|OnQueryFinishedEvent_Event
  (params (QueryInstance :type Env%20Query%20Instance%20Blueprint%20Wrapper%20Object%20Reference) (QueryStatus :type EEnvQueryStatus%20Enum :default "Processing"))
  (switch Utilities|FlowControl|Switch|SwitchonEEnvQueryStatus QueryStatus
    (:Success
      (bind _resultlocations (AI|EQS|GetQueryResultsasLocations QueryInstance))
      (for _array_element _resultlocations
        (Game|SpawnActorfromClass (select (Math|Random|RandomBoolwithWeight 0.5) "/Game/Blueprints/AI/BP_AdvanceAI.BP_AdvanceAI_C" "/Game/Blueprints/AI/BP_TrackerBot.BP_TrackerBot_C") (Math|Transform|MakeTransform _array_element) "AdjustIfPossibleButDontSpawnIfColliding" 0 0)))))

(event Custom|OnActorKilled_Event_0
  (params (VictimActor :type Actor%20Object%20Reference) (KillerActor :type Actor%20Object%20Reference) (KillerController :type Controller%20Object%20Reference))
  (Utilities|IsValid KillerController
    (:Is%20Valid
      (bind _asbp_advance_ai (Utilities|Casting|CastToBP_AdvanceAI VictimActor)
        (:then
          (Variables|Default|SetKillScore (Math|Conversions|ToFloat(Byte) (Variables|/Script/CoopGame.CoopGameCharacter|GetKilledScore _asbp_advance_ai))))
        (:CastFailed
          (bind _astracker_bot (Utilities|Casting|CastToTrackerBot VictimActor))
          (Variables|Default|SetKillScore (Math|Conversions|ToFloat(Byte) (Variables|/Script/CoopGame.TrackerBot|GetKilledScore _astracker_bot)))))
      (bind _ascoop_player_state (Utilities|Casting|CastToCOOP_PlayerState (Variables|/Script/Engine.Pawn|GetPlayerState (Pawn|GetControlledPawn KillerController))))
      (Class|COOPPlayerState|AddScore _ascoop_player_state (Variables|Default|GetKillScore))
      (Development|PrintString (Utilities|String|ToString(Float) (Variables|/Script/Engine.PlayerState|GetScore _ascoop_player_state)) true true "(R=0.000000,G=0.500000,B=0.000000,A=1.000000)"))))

(event EventBeginPlay
  (|CallParentFunction)
  (EventDispatchers|AssignOnActorKilled (delegate Custom|OnActorKilled_Event_0)))

(event EventOnRestartPlayer
  (params (NewPlayer :type Controller%20Object%20Reference))
  (|CallParentFunction NewPlayer)
  (bind _asbp_player_character (Utilities|Casting|CastToBP_PlayerCharacter (Pawn|GetControlledPawn NewPlayer)))
  (Default|CreateHUD _asbp_player_character))

(event EventSpawnNewBot
  (bind _returnvalue (AI|EQS|RunEQSQuery "/Game/Blueprints/AI/EQS_FindSpawnLocation.EQS_FindSpawnLocation" self "RandomBest25Pct"))
  (EventDispatchers|AssignOnQueryFinishedEvent _returnvalue (delegate Custom|OnQueryFinishedEvent_Event)))

(fn ConstructionScript
  (|CallParentFunction))