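; Behavior Tree decorator that gates a branch on how far the AI pawn is from an actor stored in the Blackboard.
; It reads the actor from a configurable key and passes when the straight-line distance between the two locations is at least DistanceToCheck.
; It fails when the key holds no valid actor.
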(fn PerformConditionCheckAI
  (params (OwnerController :type AI%20Controller%20Object%20Reference) (ControlledPawn :type Pawn%20Object%20Reference))
  (bind _bb_key (Variables|Default|GetBB_Key))
  (bind _returnvalue (AI|BehaviorTree|GetBlackboardValueasActor _bb_key))
  (Utilities|IsValid _returnvalue
    (:Is%20Valid
      (return (>= (Math|Vector|VectorLength (- (Transformation|GetActorLocation ControlledPawn) (Transformation|GetActorLocation _returnvalue))) (Variables|Default|GetDistanceToCheck))))
    (:Is%20Not%20Valid
      (return false))))