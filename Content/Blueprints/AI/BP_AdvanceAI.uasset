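; BP_AdvanceAI is an AI-controlled actor that runs the BT_AdvanceAI behavior tree.
; On BeginPlay it starts the tree through its AI controller and sets the isDead blackboard key to false.
; When its HealthComponent reports health at or below zero, it sets isDead to true, leaving any death response outside this Blueprint.
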(event OnHealthChanged(HealthComponent)
  (params (HealthComp :type FPS%20Health%20Component%20Object%20Reference) (Health :type Float%20%28single-precision%29) (Damage :type Float%20%28single-precision%29) (DamageType :type Damage%20Type%20Object%20Reference) (InstigatedBy :type Controller%20Object%20Reference) (DamageCauser :type Actor%20Object%20Reference))
  (bind _self self)
  (bind _returnvalue (AI|GetAIController _self))
  (bind _returnvalue_2 (AI|GetBlackboard _returnvalue))
  (if (<= Health 0.0)
    (Utilities|IsValid _returnvalue_2
      (:Is%20Valid
        (AI|Components|Blackboard|SetValueasBool _returnvalue_2 (Utilities|Name|MakeLiteralName "isDead") true)))))

(event EventBeginPlay
  (bind _self self)
  (bind _returnvalue (AI|GetAIController _self))
  (|CallParentFunction)
  (Utilities|IsValid _returnvalue
    (:Is%20Valid
      (AI|RunBehaviorTree _returnvalue "/Game/Blueprints/AI/BT_AdvanceAI.BT_AdvanceAI")
      (AI|Components|Blackboard|SetValueasBool (AI|GetBlackboard _returnvalue) (Utilities|Name|MakeLiteralName "isDead") false))))

(fn ConstructionScript
  (|CallParentFunction))